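; Goose game board actor that holds the ordered squares and answers queries about them by index.
; An editor-run FillCell event rebuilds the Box array from directly attached BP_Box actors, placing each at its own Index.
; GetBoxPosition returns a square's world location for player movement, or prints an error and returns zero if invalid.
; GetBoxMove returns the Move value of the square's BP_Bonus component, or 0 without one.
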(event `FillCell`
  ; Remplie la map Box quand on appuie sur fillcell en editor
  (`KismetArrayLibrary.Array_Clear` (`self.Box`))
  (for _array_element (`self.GetAttachedActors` true)
    (bind _asbp_box (cast `/Game/GooseGame/BP/BP_Box` _array_element))
    (`KismetArrayLibrary.Array_Set` (`self.Box`) (`/Game/GooseGame/BP/BP_Box.Index` _asbp_box) _asbp_box true)))

(fn `GetBoxMove`
  (params (Index :type Integer))
  (returns (Move :type Integer))
  (bind _returnvalue (`self.GetComponentByClass` (`|GetArrayItem` (`self.Box`) Index) "/Game/GooseGame/BP/Bonus/BP_Bonus.BP_Bonus_C"))
  ; Donne la position du joueur
  ; rend le Nombre accroché à move dans BP_Bonus
  (`/Engine/EditorBlueprintResources/StandardMacros.IsValid` _returnvalue
    (:`Is Valid`
      (return (`/Game/GooseGame/BP/Bonus/BP_Bonus.Move` _returnvalue)))
    (:`Is Not Valid`
      ; rend 0 si pas de component BP_Bonus
      (return 0))))

(fn `GetBoxPosition`
  (params (Index :type Integer))
  (returns (Position :type "Vector Structure"))
  (bind _output (`|GetArrayItem` (`self.Box`) Index))
  ; récupère la position de la prochaine case
  (`/Engine/EditorBlueprintResources/StandardMacros.IsValid` _output
    (:`Is Valid`
      (return (`self.K2_GetActorLocation` _output)))
    (:`Is Not Valid`
      (`KismetSystemLibrary.PrintString` "Case n'existe pas")
      (return (0.0 0.0 0.0)))))

(fn `UserConstructionScript`)