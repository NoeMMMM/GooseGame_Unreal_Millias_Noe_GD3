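; Player pawn for a Game of the Goose board game, walking box by box according to the dice result.
; Binds to the Dice result event, then a recursive delayed Step updates the position index in GI_GooseGame, with direction reversal at box 63.
; On stopping, the Board's box move can trigger another walk; landing on 63 otherwise prints a win and resets to 0.
; Tick interpolates the actor at constant speed toward the box position supplied by Board.
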(event `self.ReceiveBeginPlay`
  ; Récupère event dispatcher depuis dice
  (add `/Game/GooseGame/BP/BP_Dice.OnResult` (`self.Dice`) (`|CreateDelegate` :!event `RollResult`))
  ; set position de départ sur la position du joueur
  (set `self.Target` (`self.K2_GetActorLocation`))
  ; Appelle la game instance pour récupérer PositionGI
  (bind _asgi_goose_game (cast `/Game/GooseGame/BP/GameInstant/GI_GooseGame` (`GameplayStatics.GetGameInstance`)))
  (set `self.As GI Goose Game` _asgi_goose_game))

(event `RollResult`
  (params (result :type Integer))
  ; Annonce le resultat du dé et lance l'avancer du pion
  (if (not (`self.IsMoving`))
    (set `self.IsMoving` true)
    (`self.Walk` result)))

(event `Walk`
  (params (Steps :type Integer))
  ; Set la distance que devra marcher le pion
  (set `self.Direction` 1)
  (if (< Steps 0)
    (set `self.Direction` -1)
    (set `self.MovementLeft` (`KismetMathLibrary.Abs_Int` Steps))
    (`self.Step`)
    (else
      (set `self.MovementLeft` Steps)
      (`self.Step`))))

(event `Step`
  ; Bouge le pion
  ;; Si c'est la dernière case et qu'il reste du mouvement fais demi tour
  (if (and (== (`/Game/GooseGame/BP/GameInstant/GI_GooseGame.PositionGI` (`self.As GI Goose Game`)) 63) (== (`self.MovementLeft`) 1))
    ;; Le pion ne peut pas reculer plus loin que la case de départ
    (set `self.Direction` -1))
  (if (and (== (`/Game/GooseGame/BP/GameInstant/GI_GooseGame.PositionGI` (`self.As GI Goose Game`)) 0) (== (`self.MovementLeft`) -1))
    (`self.Stop Walk`)
    (else
      (bind _output_get (set `/Game/GooseGame/BP/GameInstant/GI_GooseGame.PositionGI` (+ (`/Game/GooseGame/BP/GameInstant/GI_GooseGame.PositionGI` (`self.As GI Goose Game`)) (`self.Direction`)) (`self.As GI Goose Game`)))
      (`self.MoveTo`)
      (`KismetSystemLibrary.PrintString` (`KismetStringLibrary.Conv_IntToString` _output_get))
      (`KismetSystemLibrary.Delay` 0.5)
      (set `self.MovementLeft` (- (`self.MovementLeft`) 1))
      (if (> (`self.MovementLeft`) 0)
        (`self.Step`)
        (else
          (`self.Stop Walk`))))))

(event `Stop Walk`
  ; Stop la marche
  ;; Vérifie si la case de l'arret est une case bonus ou malus
  (bind _move (`/Game/GooseGame/BP/BP_Board.GetBoxMove` (`self.Board`) (`/Game/GooseGame/BP/GameInstant/GI_GooseGame.PositionGI` (`self.As GI Goose Game`))))
  (if (== _move 0)
    (if (== (`/Game/GooseGame/BP/GameInstant/GI_GooseGame.PositionGI` (`self.As GI Goose Game`)) 63)
      (`KismetSystemLibrary.PrintString` "You win ")
      (set `/Game/GooseGame/BP/GameInstant/GI_GooseGame.PositionGI` 0 (`self.As GI Goose Game`))
      (`self.MoveTo`)
      (`KismetSystemLibrary.Delay` 1.0))
    (set `self.IsMoving` false)
    (`KismetSystemLibrary.PrintString` "Fin de la marche")
    (else
      (`KismetSystemLibrary.Delay` 1.0)
      (`self.Walk` _move)
      (`KismetSystemLibrary.PrintString` "et on repart"))))

(event `MoveTo`
  ; récupère la nouvelle position pour le pion
  (bind _position (`/Game/GooseGame/BP/BP_Board.GetBoxPosition` (`self.Board`) (`/Game/GooseGame/BP/GameInstant/GI_GooseGame.PositionGI` (`self.As GI Goose Game`))))
  (set `self.Target` _position))

(event `self.ReceiveTick`
  (params (DeltaSeconds :type "Float (single-precision)"))
  ; Fais bouger le pion vers la nouvelle position (à optimiser)
  (`self.K2_SetActorLocation` (`KismetMathLibrary.VInterpTo_Constant` (`self.K2_GetActorLocation`) (`self.Target`) DeltaSeconds (`self.MoveSpeed`))))

(fn `UserConstructionScript`)