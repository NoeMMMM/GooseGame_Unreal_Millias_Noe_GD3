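; BP_Dice is a dice actor for the goose game that rolls a random number from one to six.
; On BeginPlay it binds its Roll event to a roll dispatcher on the player's BP_TopDownCharacter.
; Roll prints the result, waits briefly, then broadcasts it through the OnResult dispatcher, with an IsRolling flag blocking overlapping rolls.
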(event `self.ReceiveBeginPlay`
  ; crée event roll
  (bind _asbp_top_down_character (cast `/Game/TopDown/Blueprints/BP_TopDownCharacter` (`GameplayStatics.GetPlayerCharacter` 0)))
  (add `/Game/TopDown/Blueprints/BP_TopDownCharacter.Roll` _asbp_top_down_character (`|CreateDelegate` :!event `Roll`)))

(event `Roll`
  ; Lance le dé et envoie le résultat
  (if (not (`self.Is rolling`))
    (set `self.Is rolling` true)
    (set `self.Result` (`KismetMathLibrary.RandomIntegerInRange` 1 6))
    (`KismetSystemLibrary.PrintString` (`KismetStringLibrary.Conv_IntToString` (`self.Result`)))
    (`KismetSystemLibrary.Delay` 1.0)
    (`self.OnResult` (`self.Result`))
    (set `self.Is rolling` false)))

(fn `UserConstructionScript`)